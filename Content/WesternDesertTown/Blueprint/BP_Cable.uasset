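; BP_Cable is a spline-driven cable prop that lays the SM_Cable mesh along an editable spline.
; The construction script divides the spline length by MeshLength and adds one spline mesh per whole segment, leaving any shorter remainder uncovered.
; Each segment takes local positions and tangents from the spline, with tangent size clamped to MeshLength.
; The event graph holds only disabled placeholder events, so it adds no runtime logic.
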(event EventBeginPlay)

(event Collision|EventActorBeginOverlap
  (params (OtherActor :type Actor%20Object%20Reference)))

(event EventTick
  (params (DeltaSeconds :type Float%20%28single-precision%29)))

(fn ConstructionScript
  (bind _spline (Variables|Default|GetSpline))
  (bind _output_get (Variables|Default|Setmesh%20count (Math|Float|Truncate (/ (Spline|GetSplineLength (Variables|Default|GetSpline)) (Variables|Default|GetMesh%20length)))))
  (for _index (range 0 (- _output_get 1))
    (bind _returnvalue (AddComponent|AddSplineMeshComponent false))
    (SplineMesh|SetStartandEnd _returnvalue (Spline|GetLocationatDistanceAlongSpline _spline (* _index (Variables|Default|GetMesh%20length)) "Local") (Math|Vector|ClampVectorSize (Spline|GetTangentatDistanceAlongSpline _spline (* _index (Variables|Default|GetMesh%20length)) "Local") 0.0 (Variables|Default|GetMesh%20length)) (Spline|GetLocationatDistanceAlongSpline _spline (* (+ _index 1) (Variables|Default|GetMesh%20length)) "Local") (Math|Vector|ClampVectorSize (Spline|GetTangentatDistanceAlongSpline _spline (* (+ _index 1) (Variables|Default|GetMesh%20length)) "Local") 0.0 (Variables|Default|GetMesh%20length)) true :!class /Script/Engine.SplineMeshComponent)
    (Components|StaticMesh|SetStaticMesh _returnvalue "/Game/WesternDesertTown/Mesh/Telegraph/SM_Cable.SM_Cable")))