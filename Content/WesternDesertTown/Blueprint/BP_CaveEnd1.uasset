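; BP_CaveEnd1 is a configurable cave end piece from the WesternDesertTown content, assembled entirely in its construction script.
; Ceiling and wall decoration selectors assign static meshes for beams, supports and decoration variants, with Option 2 in each also including the beams or supports.
; Toggles show three direction visualizers and dust particles, whose density feeds a particle parameter.
; The event graph holds only disabled placeholder events, so it adds no runtime logic.
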(event EventBeginPlay)

(event Collision|EventActorBeginOverlap
  (params (OtherActor :type Actor%20Object%20Reference)))

(event EventTick
  (params (DeltaSeconds :type Float%20%28single-precision%29)))

(fn ConstructionScript
  (bind _particles (Variables|Default|GetParticles))
  (bind _visualize_direction (Variables|Default|GetVisualize%20Direction))
  (Utilities|FlowControl|Sequence
    (:then_0
      (Utilities|FlowControl|Sequence
        (:then_0
          (Rendering|SetVisibility (Variables|Default|GetDirection1) _visualize_direction false))
        (:then_1
          (Rendering|SetVisibility (Variables|Default|GetDirection2) _visualize_direction false))
        (:then_2
          (Rendering|SetVisibility (Variables|Default|GetDirection3) _visualize_direction false))))
    (:then_1
      (switch Utilities|FlowControl|Switch|SwitchonENUM_CeilingType (Variables|Default|GetCeiling%20Decoration)
        (:NewEnumerator1
          (Components|StaticMesh|SetStaticMesh (Variables|Default|GetBeams) "/Game/WesternDesertTown/Mesh/CaveModules/CaveSupport/SM_End01Beams.SM_End01Beams" :!label _label))
        (:NewEnumerator2
          (Utilities|FlowControl|Sequence
            (:then_0
              (goto _label))
            (:then_1
              (Components|StaticMesh|SetStaticMesh (Variables|Default|GetCeilingDecoration) "/Game/WesternDesertTown/Mesh/CaveModules/CaveDecoration/SM_End01Ceiling01.SM_End01Ceiling01" :!label _label_2))))
        (:NewEnumerator3
          (goto _label_2))
        (:NewEnumerator4
          (Components|StaticMesh|SetStaticMesh (Variables|Default|GetCeilingDecoration) "/Game/WesternDesertTown/Mesh/CaveModules/CaveDecoration/SM_End01Ceiling02.SM_End01Ceiling02")
          (Components|StaticMesh|SetStaticMesh (Variables|Default|GetBeams) "/Game/WesternDesertTown/Mesh/CaveModules/CaveSupport/SM_End01Beams.SM_End01Beams"))))
    (:then_2
      (switch Utilities|FlowControl|Switch|SwitchonENUM_WallsType (Variables|Default|GetWall%20Decoration)
        (:NewEnumerator1
          (Components|StaticMesh|SetStaticMesh (Variables|Default|GetSupports) "/Game/WesternDesertTown/Mesh/CaveModules/CaveSupport/SM_End01Supports.SM_End01Supports" :!label _label_3))
        (:NewEnumerator2
          (Utilities|FlowControl|Sequence
            (:then_0
              (goto _label_3))
            (:then_1
              (Components|StaticMesh|SetStaticMesh (Variables|Default|GetWallsDecoration) "/Game/WesternDesertTown/Mesh/CaveModules/CaveDecoration/SM_End01Walls01.SM_End01Walls01" :!label _label_4))))
        (:NewEnumerator3
          (goto _label_4))
        (:NewEnumerator4
          (Components|StaticMesh|SetStaticMesh (Variables|Default|GetWallsDecoration) "/Game/WesternDesertTown/Mesh/CaveModules/CaveDecoration/SM_End01Walls02.SM_End01Walls02")
          (Components|StaticMesh|SetStaticMesh (Variables|Default|GetSupports) "/Game/WesternDesertTown/Mesh/CaveModules/CaveSupport/SM_End01Supports.SM_End01Supports"))))
    (:then_3
      (Utilities|FlowControl|Sequence
        (:then_0
          (Rendering|SetVisibility _particles (Variables|Default|GetEnable%20Dust%20Particles) false)
          (Effects|Components|ParticleSystem|SetFloatParameter _particles "Density" (Variables|Default|GetDust%20Particles%20Density)))))))