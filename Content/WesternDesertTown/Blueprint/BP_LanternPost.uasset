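; Lantern post prop with two flickering flames, each a point light paired with a Niagara effect, configured entirely in the construction script.
; Each light gets a dynamic light-function material with random offset and jittered blink frequency.
; Those values are read back into the paired flame's dynamic fire material, keeping light and flame flicker in sync.
; Exposed variables drive intensity, minimum blink level, flame size, particle jitter and visibility.
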(event EventBeginPlay)

(event Collision|EventActorBeginOverlap
  (params (OtherActor :type Actor%20Object%20Reference)))

(event EventTick
  (params (DeltaSeconds :type Float%20%28single-precision%29)))

(fn ConstructionScript
  (bind _particle_jitter_intensity (Variables|Default|GetParticle%20Jitter%20Intensity))
  (bind _flame_width (Variables|Default|GetFlame%20Width))
  (bind _flame_height (Variables|Default|GetFlame%20Height))
  (bind _blinking_min_level (Variables|Default|GetBlinking%20min%20level))
  (bind _niagara1 (Variables|Default|GetNiagara1))
  (bind _niagara2 (Variables|Default|GetNiagara2))
  (bind _returnvalue (Math|Float|Lerp 0.0 0.3 _particle_jitter_intensity))
  (bind _returnvalue_2 (Math|Float|Lerp 0.0 0.2 _flame_height))
  (Utilities|FlowControl|Sequence
    (:then_0
      (Utilities|FlowControl|Sequence
        (:then_0
          (bind _returnvalue_3 (Rendering|Material|CreateDynamicMaterialInstance "/Game/WesternDesertTown/Material/MI_LightFunction.MI_LightFunction" "None" "None" :!class /Script/Engine.KismetMaterialLibrary))
          (Rendering|Components|Light|SetLightFunctionMaterial (Variables|Default|GetPointLight2) _returnvalue_3)
          (Rendering|Material|SetScalarParameterValue _returnvalue_3 "Random offset" (Math|Random|RandomFloatinRange 0.0 1e+02) :!class /Script/Engine.MaterialInstanceDynamic)
          (Utilities|FlowControl|Sequence
            (:then_0
              (Rendering|Material|SetScalarParameterValue _returnvalue_3 "Blinking frequency" (Math|Float|Clamp(Float) (+ (Math|Random|RandomFloatinRange 0.9 1.1) (/ (- (Variables|Default|GetBlinking%20frequency) 1e+01) 1e+01)) 0.0 1.8e+02) :!class /Script/Engine.MaterialInstanceDynamic)
              (Utilities|FlowControl|Sequence
                (:then_0
                  (Rendering|Material|SetScalarParameterValue _returnvalue_3 "Blinking min level" _blinking_min_level :!class /Script/Engine.MaterialInstanceDynamic)
                  (Rendering|Components|Light|SetIntensity (Variables|Default|GetPointLight2) (Variables|Default|GetLight%20Intensity))
                  (Rendering|SetVisibility (Variables|Default|GetPointLight2) (Variables|Default|GetEnable%20flame) false))
                (:then_1
                  (bind _returnvalue_4 (Rendering|Material|GetScalarParameterValue _returnvalue_3 "Blinking frequency" :!class /Script/Engine.MaterialInstanceDynamic)))))
            (:then_1
              (bind _returnvalue_5 (Rendering|Material|GetScalarParameterValue _returnvalue_3 "Random offset" :!class /Script/Engine.MaterialInstanceDynamic)))))
        (:then_1
          (bind _returnvalue_6 (Rendering|Material|CreateDynamicMaterialInstance "/Game/WesternDesertTown/Material/MI_LightFunction.MI_LightFunction" "None" "None" :!class /Script/Engine.KismetMaterialLibrary))
          (Rendering|Components|Light|SetLightFunctionMaterial (Variables|Default|GetPointLight1) _returnvalue_6)
          (Rendering|Material|SetScalarParameterValue _returnvalue_6 "Random offset" (Math|Random|RandomFloatinRange 0.0 1e+02) :!class /Script/Engine.MaterialInstanceDynamic)
          (Utilities|FlowControl|Sequence
            (:then_0
              (Rendering|Material|SetScalarParameterValue _returnvalue_6 "Blinking frequency" (Math|Float|Clamp(Float) (+ (Math|Random|RandomFloatinRange 0.9 1.1) (/ (- (Variables|Default|GetBlinking%20frequency) 1e+01) 1e+01)) 0.0 1.8e+02) :!class /Script/Engine.MaterialInstanceDynamic)
              (Utilities|FlowControl|Sequence
                (:then_0
                  (Rendering|Material|SetScalarParameterValue _returnvalue_6 "Blinking min level" _blinking_min_level :!class /Script/Engine.MaterialInstanceDynamic)
                  (Rendering|Components|Light|SetIntensity (Variables|Default|GetPointLight1) (Variables|Default|GetLight%20Intensity))
                  (Rendering|SetVisibility (Variables|Default|GetPointLight1) (Variables|Default|GetEnable%20flame) false))
                (:then_1
                  (bind _returnvalue_7 (Rendering|Material|GetScalarParameterValue _returnvalue_6 "Blinking frequency" :!class /Script/Engine.MaterialInstanceDynamic)))))
            (:then_1
              (bind _returnvalue_8 (Rendering|Material|GetScalarParameterValue _returnvalue_6 "Random offset" :!class /Script/Engine.MaterialInstanceDynamic)))))))
    (:then_1
      (Utilities|FlowControl|Sequence
        (:then_0
          (bind _returnvalue_9 (Rendering|Material|CreateDynamicMaterialInstance "/Game/WesternDesertTown/Material/MI_Fire.MI_Fire" "None" "None" :!class /Script/Engine.KismetMaterialLibrary))
          (Class|NiagaraComponent|SetVariableMaterial _niagara1 "Material" _returnvalue_9)
          (Niagara|SetNiagaraVariable(Float) _niagara1 "Radius" _returnvalue)
          (Niagara|SetNiagaraVariable(Float) _niagara1 "Flame Width" _flame_width)
          (Niagara|SetNiagaraVariable(Float) _niagara1 "Flame Height" _returnvalue_2)
          (Rendering|Material|SetScalarParameterValue _returnvalue_9 "Random offset" _returnvalue_8 :!class /Script/Engine.MaterialInstanceDynamic)
          (Rendering|Material|SetScalarParameterValue _returnvalue_9 "Blinking frequency" _returnvalue_7 :!class /Script/Engine.MaterialInstanceDynamic)
          (Rendering|Material|SetScalarParameterValue _returnvalue_9 "Blinking min level" _blinking_min_level :!class /Script/Engine.MaterialInstanceDynamic)
          (Rendering|Material|SetScalarParameterValue _returnvalue_9 "Particle intensity" (Variables|Default|GetParticle%20intensity) :!class /Script/Engine.MaterialInstanceDynamic)
          (Rendering|SetVisibility (Variables|Default|GetNiagara1) (Variables|Default|GetEnable%20flame) false))
        (:then_1
          (bind _returnvalue_10 (Rendering|Material|CreateDynamicMaterialInstance "/Game/WesternDesertTown/Material/MI_Fire.MI_Fire" "None" "None" :!class /Script/Engine.KismetMaterialLibrary))
          (Class|NiagaraComponent|SetVariableMaterial _niagara2 "Material" _returnvalue_10)
          (Niagara|SetNiagaraVariable(Float) _niagara2 "Radius" _returnvalue)
          (Niagara|SetNiagaraVariable(Float) _niagara2 "Flame Width" _flame_width)
          (Niagara|SetNiagaraVariable(Float) _niagara2 "Flame Height" _returnvalue_2)
          (Rendering|Material|SetScalarParameterValue _returnvalue_10 "Random offset" _returnvalue_5 :!class /Script/Engine.MaterialInstanceDynamic)
          (Rendering|Material|SetScalarParameterValue _returnvalue_10 "Blinking frequency" _returnvalue_4 :!class /Script/Engine.MaterialInstanceDynamic)
          (Rendering|Material|SetScalarParameterValue _returnvalue_10 "Blinking min level" _blinking_min_level :!class /Script/Engine.MaterialInstanceDynamic)
          (Rendering|Material|SetScalarParameterValue _returnvalue_10 "Particle intensity" (Variables|Default|GetParticle%20intensity) :!class /Script/Engine.MaterialInstanceDynamic)
          (Rendering|SetVisibility (Variables|Default|GetNiagara2) (Variables|Default|GetEnable%20flame) false))))))